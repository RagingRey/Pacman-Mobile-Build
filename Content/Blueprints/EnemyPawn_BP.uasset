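; Enemy pawn for a Pac-Man game that chases the player and restarts the current level on contact.
; It idles briefly at BeginPlay, then hunts; state-change events update AI movement, stopping when Idle and otherwise moving to the player pawn.
; A sphere hit moves Pac-Man far out of play, then reloads the level after a delay.
; IncreaseDifficulty raises movement speed in tiers by the game mode's level number.
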(event `Event State Change Setup`
  (add `self.StateChangedEvent` (delegate `Event State Change`)))

(event `Event State Change` :!signature `self.StateChangedEvent`
  (params (NameState :type "EEnemyState Enum" :default "Default"))
  (`self.UpdateMovementTarget`))

(event `self.ReceiveBeginPlay`
  (`self.Event State Change Setup`)
  (`self.Idle`)
  (`KismetSystemLibrary.Delay` 1.5)
  (`self.Hunt`))

(event `self.Sphere.OnComponentHit`
  (params (HitComponent :type "PrimitiveComponent Object Reference") (OtherActor :type "Actor Object Reference") (OtherComp :type "PrimitiveComponent Object Reference") (NormalImpulse :type "Vector Structure") (Hit :type "HitResult Structure (by ref)"))
  (bind _aspacman_pawn_bp (cast `/Game/Blueprints/PacmanPawn_BP` OtherActor))
  (`self.K2_SetActorLocation` _aspacman_pawn_bp (0.0 0.0 10000.0) false false)
  (`KismetSystemLibrary.Delay` 2.0)
  (bind _returnvalue (`GameplayStatics.GetCurrentLevelName` true))
  (`GameplayStatics.OpenLevel` (`KismetStringLibrary.Conv_StringToName` _returnvalue)))

(event `Increase Difficulty`
  ;[1 1 1] Increase Difficulty
  (bind _aspacman_game_mode_bp (cast `/Game/Blueprints/Pacman_GameMode_BP` (`GameplayStatics.GetGameMode`)))
  (bind _level_number (`/Game/Blueprints/Pacman_GameMode_BP.Level Number` _aspacman_game_mode_bp))
  (if (> _level_number 6)
    (set `FloatingPawnMovement.MaxSpeed` 800.0 (`self.FloatingPawnMovement`))
    (elif (> _level_number 4)
      (set `FloatingPawnMovement.MaxSpeed` 700.0 (`self.FloatingPawnMovement`))
      (elif (> _level_number 2)
        (set `FloatingPawnMovement.MaxSpeed` 600.0 (`self.FloatingPawnMovement`))))))

(fn `UpdateMovementTarget`
  (locals (`AI Controller` :type "AIController Object Reference"))
  (set `local.AI Controller` (`AIBlueprintHelperLibrary.GetAIController` (`self.GetController`)))
  (switch `EEnemyState` (`self.EnemyState`)
    (:`Default`
      (`AIController.MoveToActor` (`local.AI Controller`) (`GameplayStatics.GetPlayerPawn` 0) -0.0 false true true null true))
    (:`Idle`
      (`Controller.StopMovement` (`local.AI Controller`)))))

(fn `UserConstructionScript`)