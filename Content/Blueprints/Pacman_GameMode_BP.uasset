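; Game mode for a Pac-Man game that sets up each level and advances play when all food is gone.
; BeginPlay blends to the first placed CameraActor, adds the HUD and unfreezes the Pac-Man pawn after a short delay.
; Tick counts Food actors; at zero it shows a win widget every tick until a delayed level change.
; A hardcoded name chain opens Level_02 through Level_10, then MainMenu, before calling IncreaseDifficulty on one enemy.
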(event `self.ReceiveBeginPlay`
  (`self.InitializeCamera`)
  (`self.Add Widget`)
  (`KismetSystemLibrary.Delay` 2.0)
  (bind _aspacman_pawn_bp (cast `/Game/Blueprints/PacmanPawn_BP` (`GameplayStatics.GetPlayerPawn` 0)))
  (`PacmanPawn.SetFrozen` _aspacman_pawn_bp false))

(event `self.ReceiveTick`
  (params (DeltaSeconds :type "Float (single-precision)"))
  (`self.Get Food`)
  (`self.You WIn`))

(event `InitializeCamera`
  ;[1 1 1] Find And Initiate Camera
  (bind _outactors (`GameplayStatics.GetAllActorsOfClass` "/Script/Engine.CameraActor"))
  (`PlayerController.SetViewTargetWithBlend` (`GameplayStatics.GetPlayerController` 0) (`|GetArrayItem` _outactors) 1.0 "VTBlend_Linear" 0.0 false))

(event `Add Widget`
  ;[1 1 1] Add Pacman UI Widget
  (bind _returnvalue (`|CreateWidget` "/Game/Blueprints/UI/Pacman_Widget_BP.Pacman_Widget_BP_C"))
  (`UserWidget.AddToViewport` _returnvalue 0))

(event `Get Food`
  ;[1 1 1] Get Food Count
  (bind _outactors (`GameplayStatics.GetAllActorsOfClass` "/Script/Pacman.Food"))
  (set `self.Foods Remaining` (`KismetArrayLibrary.Array_Length` _outactors)))

(event `You WIn`
  ;[1 1 1] If Player Wins
  (bind _output_get (set `self.Foods Remaining` (`self.Foods Remaining`)))
  (bind _output_get_2 (set `self.No Food` (== _output_get 0)))
  (if _output_get_2
    (bind _returnvalue (`|CreateWidget` "/Game/Blueprints/UI/YouWin_Widget_BP.YouWin_Widget_BP_C"))
    (`UserWidget.AddToViewport` _returnvalue 0)
    (`KismetSystemLibrary.Delay` 3.0)
    (`self.Open Next Level`)
    (`/Engine/EditorBlueprintResources/StandardMacros.IncrementInt` (`self.Level Number`)
      (:`  `
        (bind _returnvalue_2 (`GameplayStatics.GetActorOfClass` "/Game/Blueprints/EnemyPawn_BP.EnemyPawn_BP_C"))
        (`/Game/Blueprints/EnemyPawn_BP.Increase Difficulty` _returnvalue_2)))))

(event `Open Next Level`
  ;[1 1 1] Open Next Level
  (bind _returnvalue (`GameplayStatics.GetCurrentLevelName` true))
  (bind _returnvalue_2 (`KismetStringLibrary.Conv_StringToName` _returnvalue))
  (if (== _returnvalue_2 "Level_01")
    (`GameplayStatics.OpenLevel` "Level_02")
    (elif (== _returnvalue_2 "Level_02")
      (`GameplayStatics.OpenLevel` "Level_03")
      (elif (== _returnvalue_2 "Level_03")
        (`GameplayStatics.OpenLevel` "Level_04")
        (elif (== _returnvalue_2 "Level_04")
          (`GameplayStatics.OpenLevel` "Level_05")
          (elif (== _returnvalue_2 "Level_05")
            (`GameplayStatics.OpenLevel` "Level_06")
            (elif (== _returnvalue_2 "Level_06")
              (`GameplayStatics.OpenLevel` "Level_07")
              (elif (== _returnvalue_2 "Level_07")
                (`GameplayStatics.OpenLevel` "Level_08")
                (elif (== _returnvalue_2 "Level_08")
                  (`GameplayStatics.OpenLevel` "Level_09")
                  (elif (== _returnvalue_2 "Level_09")
                    (`GameplayStatics.OpenLevel` "Level_10")
                    (elif (== _returnvalue_2 "Level_10")
                      (`GameplayStatics.OpenLevel` "MainMenu"))))))))))))

(fn `UserConstructionScript`)